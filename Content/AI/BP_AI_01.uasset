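; Melee enemy AI character that attacks with a sword and uses Gameplay Abilities for hit reactions.
; PlayAnim cycles through five attack montages, gated by IsAttack and a valid blackboard Player.
; TraceSword runs a looping timer that calls Attack from the child-actor sword's arrow until TraceStop clears it.
; DamageTaken activates GA_HitReaction, Grand initializes the ability list, and UpdateWidget pushes health to the enemy widget.
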(event `self.UpdateWidget`
  (params (cur_helth :type "Float (single-precision)") (max_helth :type "Float (single-precision)"))
  ;[0 0 0] AI Character
  ;;[0.449 1 0.1175] Update Helth UI
  (bind _returnvalue (`self.GetWidgetFromWidgetComponent`))
  (bind _aswb_enemy_ui (cast `/Game/Widgets/WB_EnemyUI` _returnvalue))
  (`/Game/Widgets/WB_EnemyUI.UpdateHelth` _aswb_enemy_ui cur_helth max_helth))

(event `TraceSword`
  ;[0 0 0] AI Character
  ;;[0.04934 0.1244 1] Attack System
  ;;;[1 0.02717 0.2379] Trace Sword
  (bind _returnvalue (`KismetSystemLibrary.K2_SetTimerDelegate` (delegate `StartTrace`) 0.1 true))
  (set `self.Timer` _returnvalue))

(event `StartTrace`
  ;[0 0 0] AI Character
  ;;[0.04934 0.1244 1] Attack System
  ;;;[1 0.02717 0.2379] Trace Sword
  (bind _asbp_sword (cast `/Game/Bluprints/BP_Sword` (`ChildActorComponent.ChildActor` (`self.BP_Sword`))))
  (`self.Attack` (`self.Mesh`) (`/Game/Bluprints/BP_Sword.Arrow` _asbp_sword) "Sword"))

(event `TraceStop`
  ;[0 0 0] AI Character
  ;;[0.04934 0.1244 1] Attack System
  ;;;[1 0.02717 0.2379] Trace Sword
  (`KismetSystemLibrary.K2_ClearAndInvalidateTimerHandle` (`self.Timer`)))

(event `self.DamageTaken`
  ;[0 0 0] AI Character
  ;;[0.04934 0.1244 1] Attack System
  ;;;[1 0.06042 0.1201] Recieve Damage
  (`/Engine/EditorBlueprintResources/StandardMacros.DoOnce` false :!label _label
    (:`Completed`
      (set `self.can_apply` false)
      (`AbilitySystemComponent.TryActivateAbilityByClass` (`self.GA_Component`) "/Game/GAS/Abbilities/GA_HitReaction.GA_HitReaction_C" true)
      (set `self.can_apply` true)
      (goto _label :!via `Reset`))))

(event `self.PlayAnim`
  ;[0 0 0] AI Character
  ;;[0.04934 0.1244 1] Attack System
  ;;;[1 0.02672 0.1164] Play Attack Animation
  (if (not (`self.is Attack`))
    (set `self.is Attack` true)
    (if (== (`self.CurAnim`) 5)
      (set `self.CurAnim` 0))
    (bind _asbp_my_character (cast `/Game/Bluprints/BP_MyCharacter` (`BlackboardComponent.GetValueAsObject` (`AIBlueprintHelperLibrary.GetBlackboard` null) "Player")))
    (bind _output_get (set `self.target_object` _asbp_my_character))
    (`/Engine/EditorBlueprintResources/StandardMacros.IsValid` _output_get
      (:`Is Valid`
        (`|PlayMontage` (`self.Mesh`) (select `int` (`self.curAnim`) :`0` "/Game/Animations/Montages/attack/Standing_Melee_Attack_Downward_Montage.Standing_Melee_Attack_Downward_Montage" :`1` "/Game/Animations/Montages/attack/Standing_Melee_Attack_Horizontal_Montage.Standing_Melee_Attack_Horizontal_Montage" :`2` "/Game/Animations/Montages/attack/Standing_Melee_Attack_Backhand_Montage.Standing_Melee_Attack_Backhand_Montage" :`3` "/Game/Animations/Montages/attack/Great_Sword_High_Spin_Attack_Montage.Great_Sword_High_Spin_Attack_Montage" :`4` "/Game/Animations/Montages/attack/Standing_Melee_Run_Jump_Attack_Montage.Standing_Melee_Run_Jump_Attack_Montage" :!type "AnimMontage Object Reference")
          (:`OnCompleted`
            (`/Engine/EditorBlueprintResources/StandardMacros.IncrementInt` (`self.CurAnim`)
              (:`  `
                (set `self.is Attack` false)
                (`self.EnableInput` null))))
          (:`OnInterrupted`
            (set `self.is Attack` false)))))))

(event `self.Grand`
  (for _array_element (`self.Abilities`)
    (`self.InitializeAbility` _array_element)))

(fn `Destroy Actor Now`
  (`self.K2_DestroyActor` self)
  (return))

(fn `UserConstructionScript`)