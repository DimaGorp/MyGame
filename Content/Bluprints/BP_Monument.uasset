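; BP_Monument is an interactable monument that holds a sword and offers it to the player character.
; While the sword component exists, overlapping the Col component toggles interaction on BP_MyCharacter and sets or clears its AttacedWeapon and Monument references.
; DestroySword removes the sword component, after which the validity checks stop the monument offering interaction.
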(event `self.col.OnComponentBeginOverlap`
  (params (OverlappedComponent :type "PrimitiveComponent Object Reference") (OtherActor :type "Actor Object Reference") (OtherComp :type "PrimitiveComponent Object Reference") (OtherBodyIndex :type Integer) (bFromSweep :type Boolean) (SweepResult :type "HitResult Structure (by ref)"))
  (`/Engine/EditorBlueprintResources/StandardMacros.IsValid` (`self.BP_Sword`)
    (:`Is Valid`
      (bind _asbp_my_character (cast `/Game/Bluprints/BP_MyCharacter` OtherActor))
      (`/Game/Bluprints/BP_MyCharacter.Itteract` _asbp_my_character true)
      (set `/Game/Bluprints/BP_MyCharacter.AttacedWeapon` "/Game/Bluprints/BP_Sword.BP_Sword_C" _asbp_my_character)
      (set `/Game/Bluprints/BP_MyCharacter.Monument` self _asbp_my_character))))

(event `self.col.OnComponentEndOverlap`
  (params (OverlappedComponent :type "PrimitiveComponent Object Reference") (OtherActor :type "Actor Object Reference") (OtherComp :type "PrimitiveComponent Object Reference") (OtherBodyIndex :type Integer))
  (`/Engine/EditorBlueprintResources/StandardMacros.IsValid` (`self.BP_Sword`)
    (:`Is Valid`
      (bind _asbp_my_character (cast `/Game/Bluprints/BP_MyCharacter` OtherActor))
      (`/Game/Bluprints/BP_MyCharacter.Itteract` _asbp_my_character false)
      (set `/Game/Bluprints/BP_MyCharacter.AttacedWeapon` null _asbp_my_character)
      (set `/Game/Bluprints/BP_MyCharacter.Monument` null _asbp_my_character))))

(fn `Destroy Sword`
  (`ActorComponent.K2_DestroyComponent` (`self.BP_Sword`))
  (return))

(fn `UserConstructionScript`)