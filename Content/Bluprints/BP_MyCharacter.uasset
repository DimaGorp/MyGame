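; Player character Blueprint that routes input to Gameplay Ability System abilities for melee combos, blocking, jumping, healing and throwing.
; Picking up a weapon attaches it to the sword socket, enabling a five-step buffered combo with timer-driven traces and motion warping.
; Takedowns warp to the enemy, play paired montages, then destroy it.
; It also draws a predicted spline-mesh throw arc with a landing decal and relays status to the player UI.
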(event `InputAction|TakeDown`
  (params (Key :type "Key Structure"))
  ;[0 0 0] Player Logic
  ;;[0 0.3001 0.3125] Action Inputs
  ;;;[0 0 1] Input TakeDown
  (:`Pressed`
    (`self.StartCheckIsBack`)))

(event `PlayAnim`
  ;[0 0 0] Player Logic
  ;;[0 0.9541 1] Play Animation
  (`/Engine/EditorBlueprintResources/StandardMacros.IsValid` (`self.EquipedWeapon`)
    (:`Is Valid`
      (`self.MotionWarp to Target`)
      (`self.SwordAttack`))))

(event `InputAction|PickUp`
  (params (Key :type "Key Structure"))
  ;[0 0 0] Player Logic
  ;;[0 0.3001 0.3125] Action Inputs
  ;;;[0 0 1] Input PickUp Event
  (:`Pressed`
    (`self.PickUP`)))

(event `PickUP`
  ;[0 0 0] Player Logic
  ;;[0.02409 0.06771 0.006279] Abbilities Systems
  ;;;[0.2529 1 0.05111] PikcUp
  (`/Engine/EditorBlueprintResources/StandardMacros.IsValid` (`self.BP_Potion`)
    (:`Is Valid`
      ;;;;[1 0.7872 0.0643] Update Potions in UI
      (bind _result (`/Engine/EditorBlueprintResources/StandardMacros.IncrementInt` (`self.count_of_potions`))
        (:`  `
          (`self.ChangePotionAmount` _result)
          (`/Game/Bluprints/BP_PostionHolder.Destroy` (`self.Holder`)))))
    (:`Is Not Valid`
      _))
  (if (`KismetSystemLibrary.IsValidClass` (`self.AttacedWeapon`))
    (`/Engine/EditorBlueprintResources/StandardMacros.IsValid` (`self.EquipedWeapon`)
      (:`Is Not Valid`
        (set `self.is_weapon_equiped` true)
        (bind _returnvalue (`|SpawnActorFromClass` (`self.AttacedWeapon`) (`SceneComponent.GetSocketTransform` (`self.Mesh`) "Sword" "RTS_World") "Undefined" "MultiplyWithRoot" null null))
        (bind _output_get (set `self.EquipedWeapon` _returnvalue))
        (`self.K2_AttachToComponent` _output_get (`self.Mesh`) "Sword" "SnapToTarget" "SnapToTarget" "SnapToTarget" true)
        (`/Engine/EditorBlueprintResources/StandardMacros.DoOnce` false
          (:`Completed`
            (`/Engine/EditorBlueprintResources/StandardMacros.IsValid` (`self.Monument`)
              (:`Is Valid`
                (`/Game/Bluprints/BP_Monument.Destroy Sword` (`self.Monument`))))))))))

(event `MotionWarp to Target`
  (bind _target_object (`self.target_object`))
  ;[0.04161 1 0.9901] Lock Attack Animation on Target
  (`/Engine/EditorBlueprintResources/StandardMacros.IsValid` _target_object
    (:`Is Valid`
      (`self.StartMWarping` "Victim" _target_object))
    (:`Is Not Valid`
      (`self.StopMWarping` "Victim"))))

(event `self.DamageTaken`
  ;[0 0 0] Player Logic
  ;;[0.1546 1 0.9502] Receive Damage
  (`/Engine/EditorBlueprintResources/StandardMacros.DoOnce` false :!label _label
    (:`Completed`
      (`AbilitySystemComponent.TryActivateAbilityByClass` (`self.GA_Component`) "/Game/GAS/Abbilities/Damage/GA_HitReaction.GA_HitReaction_C" true)
      (goto _label :!via `Reset`))))

(event `InputAction|Attack_click`
  (params (Key :type "Key Structure"))
  ;[0 0 0] Player Logic
  ;;[0 0.3001 0.3125] Action Inputs
  ;;;[0.01388 0.03313 1] Input Attack
  (:`Pressed`
    (if (`|EnumEquality` (`self.AbilityType`) "NewEnumerator1")
      (`AbilitySystemBlueprintLibrary.SendGameplayEventToActor` self (struct :`TagName` "Action.Throw"))
      (set `self.AbilityType` "NewEnumerator2")
      (else
        (`self.PlayAnim`)))))

(event `self.UpdateEnemyCountUI`
  (params (enemies :type Integer))
  ;[0 0 0] Player Logic
  ;;[0 0.1832 1] UI
  ;;;[1 0.75 0] Update Amout of Potions in Player UI
  (bind _aswb_player_ui (cast `/Game/Widgets/WB_PlayerUI` (`self.UI`)))
  (`/Game/Widgets/WB_PlayerUI.OnEnemyInit` _aswb_player_ui enemies))

(event `TraceSword`
  ;[0.02078 1 0.9901] Sword Tracing
  (bind _returnvalue (`KismetSystemLibrary.K2_SetTimerDelegate` (delegate `StartTrace`) 0.1 true))
  (set `self.Timer` _returnvalue))

(event `StartTrace`
  ;[0.02078 1 0.9901] Sword Tracing
  (`self.Attack` (`self.Mesh`) (`/Game/Bluprints/BP_Sword.Arrow` (`self.EquipedWeapon`)) "Sword"))

(event `SwordAttack`
  (bind _ga_component (`self.GA_Component`))
  ;[0 0 0] Player Logic
  ;;[1 0 0] Attack System
  ;;;[0 0.8848 1] Apply Damage
  (if (`self.canUseAttackAbility?`)
    (if (`self.isAttacking?`)
      (set `self.saveAttack` true)
      (else
        (set `self.isAttacking?` true)
        (switch `int` (`self.CurAnim`) :!label _label_2
          (:`0`
            (set `self.CurAnim` 1)
            (bind _returnvalue (`AbilitySystemComponent.TryActivateAbilityByClass` _ga_component "/Game/GAS/Abbilities/Damage/GA_MeleDamageBasic_1.GA_MeleDamageBasic_1_C" true)))
          (:`1`
            (set `self.CurAnim` 2)
            (bind _returnvalue_2 (`AbilitySystemComponent.TryActivateAbilityByClass` _ga_component "/Game/GAS/Abbilities/Damage/GA_MeleDamageBasic_2.GA_MeleDamageBasic_2_C" true)))
          (:`2`
            (set `self.CurAnim` 3)
            (bind _returnvalue_3 (`AbilitySystemComponent.TryActivateAbilityByClass` _ga_component "/Game/GAS/Abbilities/Damage/GA_MeleDamageBasic_3.GA_MeleDamageBasic_3_C" true)))
          (:`3`
            (set `self.CurAnim` 4)
            (bind _returnvalue_4 (`AbilitySystemComponent.TryActivateAbilityByClass` _ga_component "/Game/GAS/Abbilities/Damage/GA_MeleDamageBasic_4.GA_MeleDamageBasic_4_C" true)))
          (:`4`
            (set `self.CurAnim` 0)
            (bind _returnvalue_5 (`AbilitySystemComponent.TryActivateAbilityByClass` _ga_component "/Game/GAS/Abbilities/Damage/GA_MeleDamageBasic_5.GA_MeleDamageBasic_5_C" true))))
        (if (not (or _returnvalue _returnvalue_2 _returnvalue_3 _returnvalue_4 _returnvalue_5))
          _)))))

(event `ChangePotionAmount`
  (params (Potion :type Integer))
  ;[0 0 0] Player Logic
  ;;[0 0.1832 1] UI
  ;;;[1 0.7638 0] Update Potion UI Icon
  (bind _aswb_player_ui (cast `/Game/Widgets/WB_PlayerUI` (`self.UI`)))
  (`/Game/Widgets/WB_PlayerUI.ChangeCountofPotionLabel` _aswb_player_ui Potion))

(event `TraceStop`
  ;[0.02078 1 0.9901] Sword Tracing
  (`KismetSystemLibrary.K2_ClearAndInvalidateTimerHandle` (`self.Timer`))
  (set `self.is_Attacking` true))

(event `Save_Attack`
  ;[0 0 0] Player Logic
  ;;[1 0 0] Attack System
  ;;;[0 0.8848 1] Apply Damage
  (if (`self.saveAttack`)
    (set `self.saveAttack` false)
    (goto _label_2)))

(event `self.UpdateUI`
  (params (cur_helth :type "Float (single-precision)") (max_helth :type "Float (single-precision)"))
  ;[1 0.8704 0] Update Helth UI
  (bind _aswb_player_ui (cast `/Game/Widgets/WB_PlayerUI` (`self.UI`)))
  (`/Game/Widgets/WB_PlayerUI.UpdateHelth` _aswb_player_ui cur_helth max_helth))

(event `Itteract`
  (params (isItteract :type Boolean))
  ;[0 0 0] Player Logic
  ;;[0 0.1832 1] UI
  ;;;[1 0.8201 0.05535] Update UI Label for Itteraction
  (bind _aswb_player_ui (cast `/Game/Widgets/WB_PlayerUI` (`self.UI`)))
  (`/Game/Widgets/WB_PlayerUI.ItteractWithObject` _aswb_player_ui isItteract))

(event `ResetCombo`
  ;[0 0 0] Player Logic
  ;;[1 0 0] Attack System
  ;;;[0 0.8848 1] Apply Damage
  (set `self.CurAnim` 0)
  (set `self.saveAttack` false)
  (set `self.isAttacking?` false)
  (`KismetSystemLibrary.PrintString` "Start"))

(event `self.TakeDown`
  (params (target :type "Actor Object Reference") (LOcation :type "Vector Structure") (Rotation :type "Rotator Structure"))
  ;[0 0 0] Player Logic
  ;;[1 0 0] Attack System
  ;;;[0.003871 0.431 0.4583] Take Down
  ;;;;[1 0.1205 0.3939] Lock Take Down on Target
  (`/Engine/EditorBlueprintResources/StandardMacros.IsValid` (`self.EquipedWeapon`)
    (:`Is Valid`
      (`/Engine/EditorBlueprintResources/StandardMacros.DoOnce` false :!label _label_3
        (:`Completed`
          (`MotionWarpingComponent.AddOrUpdateWarpTargetFromLocationAndRotation` (`self.MotionWarpComponent`) "Target" LOcation Rotation)
          ;;;;[0.03839 0.1943 1] Play Sneak Take Down Player Animation
          (bind _asbp_ai_01 (cast `/Game/AI/BP_AI_01` target))
          (`CharacterMovementComponent.DisableMovement` (`Character.CharacterMovement` _asbp_ai_01))
          (`|PlayMontage` (`self.Mesh`) "/Game/Animations/Montages/takedowns/Stab_crounch_Montage.Stab_crounch_Montage"
            (:`then`
              (`PrimitiveComponent.SetCollisionEnabled` (`Character.CapsuleComponent` _asbp_ai_01) "NoCollision")
              ;;;;[1 0 0.0578] Play Enemy Dying Animation
              (bind _returnvalue (`self.PlayAnimMontage` _asbp_ai_01 "/Game/Animations/Montages/takedowns/Dying_Montage.Dying_Montage" 1.0 "None"))
              (`KismetSystemLibrary.Delay` _returnvalue)
              (`/Game/AI/BP_AI_01.Destroy Actor Now` _asbp_ai_01)
              (`MotionWarpingComponent.RemoveWarpTarget` (`self.MotionWarpComponent`) "Target")
              (`KismetSystemLibrary.Delay` 0.2)
              ;;;;[1 0.8817 0.01873] Update UI icon
              (`self.decreasenemycount`)
              (goto _label_3 :!via `Reset`))
            (:`OnCompleted`
              (`CharacterMovementComponent.SetMovementMode` (`self.CharacterMovement`) "MOVE_Walking" 0))))))))

(event `Key|K`
  (params (Key :type "Key Structure"))
  (:`Pressed`
    (`AbilitySystemComponent.TryActivateAbilityByClass` (`self.GA_Component`) "/Game/GAS/Abbilities/Spells/GA_Healing.GA_Healing_C" false)))

(event `Key|Escape`
  (params (Key :type "Key Structure"))
  (:`Pressed`
    (bind _returnvalue (`|GenericCreateObject` "/Game/Widgets/WB_PauseUI.WB_PauseUI_C"))
    (`UserWidget.AddToViewport` _returnvalue 0)))

(event `InputAction|Block`
  (params (Key :type "Key Structure"))
  (bind _equipedweapon (`self.EquipedWeapon`))
  ;[0 0.4792 0.4792] Block
  (:`Pressed`
    (`/Engine/EditorBlueprintResources/StandardMacros.IsValid` _equipedweapon
      (:`Is Valid`
        (bind _output_get (set `self.AbilityType` "NewEnumerator4"))
        (`AbilitySystemComponent.PressInputID` (`self.GA_Component`) (`KismetMathLibrary.Conv_ByteToInt` _output_get)))))
  (:`Released`
    (`/Engine/EditorBlueprintResources/StandardMacros.IsValid` _equipedweapon
      (:`Is Valid`
        (`AbilitySystemComponent.ReleaseInputID` (`self.GA_Component`) (`KismetMathLibrary.Conv_ByteToInt` (`self.AbilityType`)))))))

(event `self.GrandAbility`
  (for (_array_element _array_index) (`self.Abbilities`)
    (`self.InitializeAbility` _array_element _array_index)))

(event `self.DealDamage`
  (params (Target :type "Actor Object Reference") (HitLocation :type "Vector Structure"))
  (`/Engine/EditorBlueprintResources/StandardMacros.IsValid` (`self.EquipedWeapon`)
    (:`Is Valid`
      (`AbilitySystemBlueprintLibrary.SendGameplayEventToActor` self (struct :`TagName` "Action.Damage") (make `GameplayEventData` (struct :`TagName` "Action.Damage") self Target)))))

(event `Key|Q`
  (params (Key :type "Key Structure"))
  (bind _returnvalue (and (not (== (`self.GetHelth`) (`self.GetMaxHelth`))) (> (`self.count_of_potions`) 0)))
  ;[0.5171 1 0.3355 1 20] Heal
  (:`Pressed`
    (bind _aswb_player_ui (cast `/Game/Widgets/WB_PlayerUI` (`self.UI`)))
    (`/Game/Widgets/WB_PlayerUI.UsePotion` _aswb_player_ui _returnvalue)
    (if _returnvalue
      (`AbilitySystemComponent.TryActivateAbilityByClass` (`self.GA_Component`) "/Game/GAS/Abbilities/Items/GA_HelingItems.GA_HelingItems_C" true)
      (set `self.isUSingPotions?` true))))

(event `Key|Z`
  (params (Key :type "Key Structure"))
  (:`Pressed`
    (bind _output_get (set `self.AbilityType` "NewEnumerator1"))
    (`AbilitySystemComponent.PressInputID` (`self.GA_Component`) (`KismetMathLibrary.Conv_ByteToInt` _output_get)))
  (:`Released`
    (`self.ReleasInputForce`)))

(event `ReleasInputForce`
  (bind _output_get (set `self.AbilityType` "NewEnumerator1"))
  (`AbilitySystemComponent.ReleaseInputID` (`self.GA_Component`) (`KismetMathLibrary.Conv_ByteToInt` _output_get)))

(event `InputAction|Jump`
  (params (Key :type "Key Structure"))
  (:`Pressed`
    (`AbilitySystemComponent.TryActivateAbilityByClass` (`self.GA_Component`) "/Game/GAS/Abbilities/Movement/GA_Jump.GA_Jump_C" true)))

(event `isLanded`
  (`AbilitySystemBlueprintLibrary.SendGameplayEventToActor` self (struct :`TagName` "Action.Jump")))

(event `FireballAbilityUI`
  (params (Activate :type Boolean))
  ;[0.3427 1 0.02544] FireballAbilityUI
  (if Activate
    (bind _aswb_player_ui (cast `/Game/Widgets/WB_PlayerUI` (`self.UI`)))
    (`/Game/Widgets/WB_PlayerUI.FireBallActivate` _aswb_player_ui)
    (else
      (bind _aswb_player_ui_2 (cast `/Game/Widgets/WB_PlayerUI` (`self.UI`)))
      (`/Game/Widgets/WB_PlayerUI.FireballDeactivate` _aswb_player_ui_2))))

(event `HealingAbilityUI`
  (params (Cooldown :type "Float (double-precision)"))
  ;[0.4114 1 0.1027] HealingAbilityUI
  (bind _aswb_player_ui (cast `/Game/Widgets/WB_PlayerUI` (`self.UI`)))
  (`/Game/Widgets/WB_PlayerUI.HealingActivate` _aswb_player_ui true Cooldown))

(event `Projectile`
  (params (Start :type "Vector Structure") (End :type "Vector Structure") (Object :type "Array of Actor Object Reference"))
  (bind _spline (`self.Spline`))
  (`self.ClearArc`)
  (bind _predictresult (`GameplayStatics.Blueprint_PredictProjectilePath_Advanced` (make `PredictProjectilePathParams` Start End true 1.0 3.0 true "ECC_WorldStatic" _ Object 100.0)))
  (`|ExecutionSequence`
    (:`then_0`
      (for (_array_element _array_index) (break `PredictProjectilePathResult` _predictresult)
        (`SplineComponent.AddSplinePointAtIndex` _spline (break `PredictProjectilePathPointData` _array_element) _array_index "World" true))
      (bind _returnvalue (`KismetArrayLibrary.Array_LastIndex` (break `PredictProjectilePathResult` _predictresult)))
      (`SplineComponent.SetSplinePointType` _spline _returnvalue "CurveClamped" true)
      (for _index (range (+ (- (`SplineComponent.GetNumberOfSplinePoints` _spline) 2) 1))
        (bind _returnvalue_2 (`AddComponent|NODE_AddSplineMeshComponent-3` :`bManualAttachment` true))
        (`SplineMeshComponent.SetStartScale` _returnvalue_2 (`KismetMathLibrary.MakeVector2D` 0.1 0.1) true)
        (`SplineMeshComponent.SetEndScale` _returnvalue_2 (`KismetMathLibrary.MakeVector2D` 0.1 0.1) true)
        (`KismetArrayLibrary.Array_Add` (`self.PointsArray`) _returnvalue_2)
        (bind _returnvalue_3 (+ _index 1))
        (`SplineMeshComponent.SetStartAndEnd` _returnvalue_2 (`.Location` (break `PredictProjectilePathPointData` (`|GetArrayItem` (break `PredictProjectilePathResult` _predictresult) _index))) (`SplineComponent.GetTangentAtSplinePoint` (`self.Spline`) _index "World") (`.Location` (break `PredictProjectilePathPointData` (`|GetArrayItem` (break `PredictProjectilePathResult` _predictresult) _returnvalue_3))) (`SplineComponent.GetTangentAtSplinePoint` (`self.Spline`) _returnvalue_3 "World") true)))
    (:`then_1`
      (`SceneComponent.K2_SetWorldLocation` (`self.Decal`) (`.Location` (break `PredictProjectilePathPointData` (`|GetArrayItem` (break `PredictProjectilePathResult` _predictresult) _returnvalue))) false true)
      (`SceneComponent.SetVisibility` (`self.Decal`) true false))))

(event `ClearArc`
  (bind _pointsarray (`self.PointsArray`))
  (`ActorComponent.K2_DestroyComponent` _pointsarray)
  (`KismetArrayLibrary.Array_Clear` _pointsarray)
  (`SplineComponent.ClearSplinePoints` (`self.Spline`) true)
  (`SceneComponent.SetVisibility` (`self.Decal`) false false))

(fn `UserConstructionScript`)