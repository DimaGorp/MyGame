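; BP_Fireball is a fireball projectile that sets enemies on fire on contact.
; The first sphere overlap with an Enemy-tagged actor applies the GE_OnFire gameplay effect to that actor's Ability System, then destroys the fireball.
; Every Tick copies Speed into the projectile movement's initial and max speed, then feeds a derived value to the particle effect's X_Velocity.
; A duplicate of this speed setup sits unconnected in the construction script.
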(event `self.Sphere Collision.OnComponentBeginOverlap`
  (params (OverlappedComponent :type "PrimitiveComponent Object Reference") (OtherActor :type "Actor Object Reference") (OtherComp :type "PrimitiveComponent Object Reference") (OtherBodyIndex :type Integer) (bFromSweep :type Boolean) (SweepResult :type "HitResult Structure (by ref)"))
  (if (`self.ActorHasTag` OtherActor "Enemy")
    (`/Engine/EditorBlueprintResources/StandardMacros.DoOnce` false
      (:`Completed`
        (`AbilitySystemComponent.BP_ApplyGameplayEffectToTarget` :`self` (`self.AbilitySystem`) :`GameplayEffectClass` "/Game/GAS/Effects/GE_OnFire.GE_OnFire_C" :`Target` (`AbilitySystemBlueprintLibrary.GetAbilitySystemComponent` OtherActor))
        (`self.K2_DestroyActor`)))))

(event `self.ReceiveTick`
  (params (DeltaSeconds :type "Float (single-precision)"))
  (bind _projectilemovement (`self.ProjectileMovement`))
  (bind _output_get (set `ProjectileMovementComponent.InitialSpeed` (`self.Speed`) _projectilemovement))
  (bind _output_get_2 (set `ProjectileMovementComponent.MaxSpeed` _output_get _projectilemovement))
  (bind _result (`/Engine/EditorBlueprintResources/StandardMacros.NegateFloat` _output_get_2)
    (:`  `
      (`NiagaraComponent.SetVariableFloat` (`self.FireBall_Particle_FX1`) "X_Velocity" _result))))

(fn `UserConstructionScript`)