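; BP_Fireball is a fire spell actor that resolves on its sphere's first relevant overlap, ignoring actors tagged Player.
; On an Enemy, a DoOnce gate applies GE_FireHittet through the Ability System, fires the FireExplosion GameplayCue at the target and destroys the fireball.
; On anything else, it line-traces 100 units down, spawns BP_FireCircles at the hit location and destroys itself.
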(event `self.Sphere.OnComponentBeginOverlap`
  (params (OverlappedComponent :type "PrimitiveComponent Object Reference") (OtherActor :type "Actor Object Reference") (OtherComp :type "PrimitiveComponent Object Reference") (OtherBodyIndex :type Integer) (bFromSweep :type Boolean) (SweepResult :type "HitResult Structure (by ref)"))
  (bind _returnvalue (`self.K2_GetActorLocation` self))
  (if (not (`self.ActorHasTag` OtherActor "Player"))
    (if (`self.ActorHasTag` OtherActor "Enemy")
      (`/Engine/EditorBlueprintResources/StandardMacros.DoOnce` false
        (:`Completed`
          (`AbilitySystemComponent.BP_ApplyGameplayEffectToTarget` :`self` (`self.AbilitySystem`) :`GameplayEffectClass` "/Game/GAS/Effects/GE_FireHittet.GE_FireHittet_C" :`Target` (`AbilitySystemBlueprintLibrary.GetAbilitySystemComponent` OtherActor))
          (`/Engine/EditorBlueprintResources/StandardMacros.IsValid` OtherActor
            (:`Is Valid`
              (`GameplayCueFunctionLibrary.ExecuteGameplayCueOnActor` OtherActor (struct :`TagName` "GameplayCue.Fire.FireExplosion") (`AbilitySystemBlueprintLibrary.MakeGameplayCueParameters` 0.0 0.0 (struct) (struct) (struct) (struct) (struct) (`self.K2_GetActorLocation` OtherActor)))))))
      (else
        (bind _outhit (`KismetSystemLibrary.LineTraceSingle` _returnvalue (- _returnvalue (0.0 0.0 100.0)) "TraceTypeQuery1"))
        (`|SpawnActorFromClass` "/Game/Bluprints/spells/BP_FireCircles.BP_FireCircles_C" (`KismetMathLibrary.MakeTransform` (`.Location` (`GameplayStatics.BreakHitResult` _outhit))) "Undefined" "MultiplyWithRoot" null null)))
    (`self.K2_DestroyActor`)))

(fn `UserConstructionScript`)