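; BP_PostionHolder is a holder actor that displays a BP_Potion child actor and offers it to BP_MyCharacter for interaction.
; Box overlaps set or clear the character's potion and holder references and toggle its interact state.
; PlayAnim ignores its Play flag, using a FlipFlop to play or reverse a timeline driving potion yaw, height and outline overlay.
; Destroy removes the potion component, which disables further overlap responses.
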(event `PlayAnim`
  (params (Play :type Boolean))
  (bind _bp_potion (`self.BP_Potion`))
  (bind _bp_potion_2 (`self.BP_Potion`))
  (bind (_relativelocation_x _relativelocation_y) (`KismetMathLibrary.BreakVector` (`SceneComponent.RelativeLocation` _bp_potion)))
  (`/Engine/EditorBlueprintResources/StandardMacros.FlipFlop`
    (:`A`
      (bind (_direction _location _rotation _color) (`Timeline|StartRotating` :!label _label)
        (:`Update`
          (`/Engine/EditorBlueprintResources/StandardMacros.IsValid` _bp_potion_2
            (:`Is Valid`
              (`SceneComponent.K2_SetRelativeRotation` _bp_potion_2 (`KismetMathLibrary.MakeRotator` 0.0 0.0 _rotation) false false)
              (`SceneComponent.K2_SetRelativeLocation` _bp_potion (`KismetMathLibrary.MakeVector` _relativelocation_x _relativelocation_y _location) false false)
              (if (> _color 0.0)
                (bind _asbp_potion (cast `/Game/Bluprints/BP_Potion` (`ChildActorComponent.ChildActor` (`self.BP_Potion`))))
                (`MeshComponent.SetOverlayMaterial` (`/Game/Bluprints/BP_Potion.Potion` _asbp_potion) "/Game/Models/potion/M_Outliner.M_Outliner")
                (else
                  (bind _asbp_potion_2 (cast `/Game/Bluprints/BP_Potion` (`ChildActorComponent.ChildActor` (`self.BP_Potion`))))
                  (`MeshComponent.SetOverlayMaterial` (`/Game/Bluprints/BP_Potion.Potion` _asbp_potion_2) null))))))))
    (:`B`
      (goto _label :!via `Reverse`))))

(event `self.Box.OnComponentBeginOverlap`
  (params (OverlappedComponent :type "PrimitiveComponent Object Reference") (OtherActor :type "Actor Object Reference") (OtherComp :type "PrimitiveComponent Object Reference") (OtherBodyIndex :type Integer) (bFromSweep :type Boolean) (SweepResult :type "HitResult Structure (by ref)"))
  (bind _asbp_my_character (cast `/Game/Bluprints/BP_MyCharacter` OtherActor))
  (`/Engine/EditorBlueprintResources/StandardMacros.IsValid` (`self.BP_Potion`)
    (:`Is Valid`
      (bind _output_get (set `self.Player` _asbp_my_character))
      (set `/Game/Bluprints/BP_MyCharacter.BP_Potion` (`self.BP_Potion`) _output_get)
      (set `/Game/Bluprints/BP_MyCharacter.Holder` self (`self.Player`))
      (`/Game/Bluprints/BP_MyCharacter.Itteract` (`self.Player`) true)
      (`self.PlayAnim` true))))

(event `self.Box.OnComponentEndOverlap`
  (params (OverlappedComponent :type "PrimitiveComponent Object Reference") (OtherActor :type "Actor Object Reference") (OtherComp :type "PrimitiveComponent Object Reference") (OtherBodyIndex :type Integer))
  (bind _asbp_my_character (cast `/Game/Bluprints/BP_MyCharacter` OtherActor))
  (`/Engine/EditorBlueprintResources/StandardMacros.IsValid` (`self.BP_Potion`)
    (:`Is Valid`
      (set `/Game/Bluprints/BP_MyCharacter.BP_Potion` null _asbp_my_character)
      (set `/Game/Bluprints/BP_MyCharacter.Holder` null (`self.Player`))
      (`/Game/Bluprints/BP_MyCharacter.Itteract` (`self.Player`) false)
      (`self.PlayAnim` false))))

(fn `Destroy`
  (`ActorComponent.K2_DestroyComponent` (`self.BP_Potion`))
  (return))

(fn `UserConstructionScript`)