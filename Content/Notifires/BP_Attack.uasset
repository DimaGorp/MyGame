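; BP_Attack is an anim notify state that drives the attack trace window for the player and AI characters during animations.
; It checks the mesh owner for the Player tag, then casts to BP_MyCharacter if tagged or BP_AI_01 otherwise.
; Begin and every tick call StartTrace on that character, and End calls TraceStop, leaving the trace logic to the character Blueprints.
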(fn `Received_NotifyBegin`
  (params (MeshComp :type "SkeletalMeshComponent Object Reference") (Animation :type "AnimSequenceBase Object Reference") (TotalDuration :type "Float (single-precision)") (EventReference :type "AnimNotifyEventReference Structure (by ref)"))
  (returns (ReturnValue :type Boolean))
  (bind _returnvalue (`ActorComponent.GetOwner` MeshComp))
  (if (`Actor.ActorHasTag` _returnvalue "PLayer")
    (bind _asbp_my_character (cast `/Game/Bluprints/BP_MyCharacter` _returnvalue))
    (`/Game/Bluprints/BP_MyCharacter.StartTrace` _asbp_my_character)
    (else
      (bind _asbp_ai_01 (cast `/Game/AI/BP_AI_01` _returnvalue))
      (`/Game/AI/BP_AI_01.StartTrace` _asbp_ai_01)))
  (return false))

(fn `Received_NotifyEnd`
  (params (MeshComp :type "SkeletalMeshComponent Object Reference") (Animation :type "AnimSequenceBase Object Reference") (EventReference :type "AnimNotifyEventReference Structure (by ref)"))
  (returns (ReturnValue :type Boolean))
  (bind _returnvalue (`ActorComponent.GetOwner` MeshComp))
  (if (`Actor.ActorHasTag` _returnvalue "Player")
    (bind _asbp_my_character (cast `/Game/Bluprints/BP_MyCharacter` _returnvalue))
    (`/Game/Bluprints/BP_MyCharacter.TraceStop` _asbp_my_character)
    (else
      (bind _asbp_ai_01 (cast `/Game/AI/BP_AI_01` _returnvalue))
      (`/Game/AI/BP_AI_01.TraceStop` _asbp_ai_01)))
  (return false))

(fn `Received_NotifyTick`
  (params (MeshComp :type "SkeletalMeshComponent Object Reference") (Animation :type "AnimSequenceBase Object Reference") (FrameDeltaTime :type "Float (single-precision)") (EventReference :type "AnimNotifyEventReference Structure (by ref)"))
  (returns (ReturnValue :type Boolean))
  (bind _returnvalue (`ActorComponent.GetOwner` MeshComp))
  (if (`Actor.ActorHasTag` _returnvalue "Player")
    (bind _asbp_my_character (cast `/Game/Bluprints/BP_MyCharacter` _returnvalue))
    (`/Game/Bluprints/BP_MyCharacter.StartTrace` _asbp_my_character)
    (else
      (bind _asbp_ai_01 (cast `/Game/AI/BP_AI_01` _returnvalue))
      (`/Game/AI/BP_AI_01.StartTrace` _asbp_ai_01)))
  (return false))