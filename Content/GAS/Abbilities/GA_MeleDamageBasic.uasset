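; Basic melee attack gameplay ability usable by both the player character and BP_AI_01, chosen by the avatar's Player tag.
; After commit it plays DamageMontage and waits once for an Action.Damage event, then applies GE_MeleDamage from the payload's instigator to its target.
; Montage completion or interruption clears IsAttacking on the Player reference, even on the AI path where that is not assigned, and ends the ability.
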(event `self.K2_ActivateAbility`
  (bind _returnvalue (`self.GetAvatarActorFromActorInfo`))
  (if (`Actor.ActorHasTag` _returnvalue "Player")
    (bind _asbp_my_character (cast `/Game/Bluprints/BP_MyCharacter` _returnvalue))
    (set `self.Player` _asbp_my_character)
    (else
      (bind _asbp_ai_01 (cast `/Game/AI/BP_AI_01` _returnvalue))
      (set `self.AI` _asbp_ai_01)))
  (bind _returnvalue_2 (`self.K2_CommitAbility`))
  (if _returnvalue_2
    (`AbilityTask_PlayMontageAndWait.CreatePlayMontageAndWaitProxy` "None" (`self.Damage Montage`)
      (:`then`
        (bind (_asynctaskproxy _payload) (`AbilityTask_WaitGameplayEvent.WaitGameplayEvent` (struct :`TagName` "Action.Damage") null true)
          (:`EventReceived`
            (bind (_eventtag _instigator _target) (break `GameplayEventData` _payload))
            (`AbilitySystemComponent.BP_ApplyGameplayEffectToTarget` :`self` (`AbilitySystemBlueprintLibrary.GetAbilitySystemComponent` _instigator) :`GameplayEffectClass` "/Game/GAS/Effects/GE_MeleDamage.GE_MeleDamage_C" :`Target` (`AbilitySystemBlueprintLibrary.GetAbilitySystemComponent` _target)))))
      (:`OnCompleted`
        (set `/Game/Bluprints/BP_MyCharacter.isAttacking?` false (`self.Player`) :!label _label)
        (`self.K2_EndAbility`))
      (:`OnInterrupted`
        (goto _label)))
    (else
      (`self.K2_EndAbility`))))