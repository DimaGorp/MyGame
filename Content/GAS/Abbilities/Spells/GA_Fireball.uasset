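; Gameplay Ability for a charged fireball spell: holding input aims, and a throw event launches a BP_Fireball.
; Activation zooms the spring arm, then a recursive delayed loop updates velocity and arc preview from control rotation while locking movement.
; An Action.Throw event plays the throw montage, whose Interrupted pin spawns the fireball at the Spells socket.
; Releasing input restores the camera and cancels unless throwing; ending clears UI and unhides the weapon.
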(event `ChargeAttack`
  (if (stale `self.K2_ActivateAbility` _output_get) :!label _label
    (bind _asbp_my_character (cast `/Game/Bluprints/BP_MyCharacter` (`self.GetAvatarActorFromActorInfo`)))
    (bind _equipedweapon (`/Game/Bluprints/BP_MyCharacter.EquipedWeapon` _asbp_my_character))
    (`/Engine/EditorBlueprintResources/StandardMacros.IsValid` _equipedweapon
      (:`Is Valid`
        (`Actor.SetActorHiddenInGame` _equipedweapon true))
      (:`Is Not Valid`
        _))
    (bind _output_get (set `self.BallVelocity` (* (`KismetMathLibrary.GetForwardVector` (`Pawn.GetControlRotation` _asbp_my_character)) (`self.Fireball Spped`))))
    (`/Game/Bluprints/BP_MyCharacter.Projectile` _asbp_my_character (`SceneComponent.GetSocketLocation` (`Character.Mesh` _asbp_my_character) "Spells") _output_get (`|MakeArray` (`self.GetAvatarActorFromActorInfo`)))
    (`KismetSystemLibrary.Delay` 0.1)
    (`AbilityTask_WaitGameplayEvent.WaitGameplayEvent` (struct :`TagName` "Action.Throw") null
      (:`then`
        (bind _ascharacter (cast `Character` (`self.GetAvatarActorFromActorInfo`)))
        (`CharacterMovementComponent.DisableMovement` (`Character.CharacterMovement` _ascharacter))
        (set `Pawn.bUseControllerRotationYaw` true _ascharacter)
        (`self.K2_AddGameplayCue` (struct :`TagName` "GameplayCue.Fire.FireBall"))
        (`self.ChargeAttack`))
      (:`EventReceived`
        (set `self.isThrowing?` true)
        (`AbilityTask_PlayMontageAndWait.CreatePlayMontageAndWaitProxy` "None" "/Game/Animations/Animation_sequnces/attack/spell/Throw_Montage.Throw_Montage"
          (:`OnInterrupted`
            (bind _ascharacter_2 (cast `Character` (`self.GetAvatarActorFromActorInfo`)))
            (set `self.isThrowing?` false)
            (`self.K2_RemoveGameplayCue` (struct :`TagName` "GameplayCue.Fire.FireBall"))
            (bind _returnvalue (`|SpawnActorFromClass` "/Game/Bluprints/spells/BP_Fireball.BP_Fireball_C" (`SceneComponent.GetSocketTransform` (`Character.Mesh` _ascharacter_2) "Spells" "RTS_World") "Undefined" "MultiplyWithRoot" null null))
            (`/Engine/EditorBlueprintResources/StandardMacros.IsValid` _returnvalue
              (:`Is Valid`
                (set `MovementComponent.Velocity` (`self.BallVelocity`) (`/Game/Bluprints/spells/BP_Fireball.ProjectileMovement` _returnvalue))
                (bind _ascharacter_3 (cast `Character` (`self.GetAvatarActorFromActorInfo`)))
                (`CharacterMovementComponent.SetMovementMode` (`Character.CharacterMovement` _ascharacter_3) "MOVE_Walking" 0)
                (set `Pawn.bUseControllerRotationYaw` false _ascharacter_3)
                (`self.K2_EndAbility`)))))))))

(event `self.K2_ActivateAbility`
  (bind _returnvalue (`self.K2_CommitAbility`))
  (if _returnvalue
    (`AbilityTask_WaitInputRelease.WaitInputRelease` false
      (:`then`
        (bind _asbp_my_character (cast `/Game/Bluprints/BP_MyCharacter` (`self.GetAvatarActorFromActorInfo`)))
        (`/Game/Bluprints/BP_MyCharacter.FireballAbilityUI` _asbp_my_character true)
        (bind _springarmcomp (`MyCharacter.SpringArmComp` _asbp_my_character))
        (set `SpringArmComponent.TargetArmLength` 250.0 _springarmcomp)
        (`SceneComponent.K2_SetRelativeLocation` _springarmcomp (50.0 0.0 150.0) false false)
        (`AbilityTask_PlayMontageAndWait.CreatePlayMontageAndWaitProxy` "None" "/Game/Animations/Animation_sequnces/attack/spell/PrepareStart_Montage.PrepareStart_Montage"
          (:`then`
            (bind _output_get (set `self.isCharging?` true))
            (goto _label))))
      (:`OnRelease`
        (bind _asbp_my_character_2 (cast `/Game/Bluprints/BP_MyCharacter` (`self.GetAvatarActorFromActorInfo`)))
        (bind _springarmcomp_2 (`MyCharacter.SpringArmComp` _asbp_my_character_2))
        (set `SpringArmComponent.TargetArmLength` 500.0 _springarmcomp_2)
        (`SceneComponent.K2_SetRelativeLocation` _springarmcomp_2 (0.0 0.0 30.0) false false)
        (if (not (`self.isThrowing?`))
          (`AbilityTask_PlayMontageAndWait.CreatePlayMontageAndWaitProxy` "None" "/Game/Animations/Animation_sequnces/attack/spell/PrepareEnd_Montage.PrepareEnd_Montage"
            (:`OnBlendOut`
              (set `self.isCharging?` false)
              (bind _ascharacter (cast `Character` (`self.GetAvatarActorFromActorInfo`)))
              (`CharacterMovementComponent.SetMovementMode` (`Character.CharacterMovement` _ascharacter) "MOVE_Walking" 0)
              (set `Pawn.bUseControllerRotationYaw` false _ascharacter)
              (`self.K2_RemoveGameplayCue` (struct :`TagName` "GameplayCue.Fire.FireBall"))
              (`self.K2_CancelAbility`))))))
    (else
      (`self.K2_EndAbility`))))

(event `self.K2_OnEndAbility`
  (params (bWasCancelled :type Boolean))
  (bind _asbp_my_character (cast `/Game/Bluprints/BP_MyCharacter` (`self.GetAvatarActorFromActorInfo`)))
  (if bWasCancelled
    (`/Game/Bluprints/BP_MyCharacter.ClearArc` _asbp_my_character)
    (`/Game/Bluprints/BP_MyCharacter.FireballAbilityUI` _asbp_my_character false))
  (bind _equipedweapon (`/Game/Bluprints/BP_MyCharacter.EquipedWeapon` _asbp_my_character))
  (`/Engine/EditorBlueprintResources/StandardMacros.IsValid` _equipedweapon
    (:`Is Valid`
      (`Actor.SetActorHiddenInGame` _equipedweapon false))
    (:`Is Not Valid`
      _))
  (`/Game/Bluprints/BP_MyCharacter.ReleasInputForce` _asbp_my_character)
  (`/Game/Bluprints/BP_MyCharacter.ClearArc` _asbp_my_character)
  (`/Game/Bluprints/BP_MyCharacter.FireballAbilityUI` _asbp_my_character false))