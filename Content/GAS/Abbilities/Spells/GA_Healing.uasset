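; Healing spell Gameplay Ability that plays a cast montage and applies GE_Healing to the avatar.
; After committing, it disables the character's movement while the montage plays and restores walking once a TimeDelayedToMove wait finishes.
; On montage completion it applies the effect, then delays by the effect's expected end time value before ending.
; A failed commit ends the ability immediately, and cancellation restores walking.
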(event `self.K2_ActivateAbility`
  (bind _returnvalue (`self.GetAvatarActorFromActorInfo`))
  (bind _returnvalue_2 (`self.K2_CommitAbility`))
  (if _returnvalue_2
    (`AbilityTask_PlayMontageAndWait.CreatePlayMontageAndWaitProxy` "None" (`self.Montage to Play`)
      (:`then`
        (bind _asbp_my_character (cast `/Game/Bluprints/BP_MyCharacter` _returnvalue))
        (set `self.Player` _asbp_my_character)
        (`AbilityTask_WaitDelay.WaitDelay` (`self.Time_Delayed_to_Move`)
          (:`then`
            (bind _charactermovement (`Character.CharacterMovement` _asbp_my_character))
            (`CharacterMovementComponent.DisableMovement` _charactermovement))
          (:`OnFinish`
            (`CharacterMovementComponent.SetMovementMode` _charactermovement "MOVE_Walking" 0))))
      (:`OnCompleted`
        (bind _returnvalue_3 (`AbilitySystemComponent.BP_ApplyGameplayEffectToSelf` :`self` (`AbilitySystemBlueprintLibrary.GetAbilitySystemComponent` _returnvalue) :`GameplayEffectClass` "/Game/GAS/Effects/GE_Healing.GE_Healing_C"))
        (bind _returnvalue_4 (`AbilitySystemBlueprintLibrary.GetActiveGameplayEffectExpectedEndTime` _returnvalue_3))
        (`KismetSystemLibrary.Delay` _returnvalue_4)
        (`self.K2_EndAbility`)))
    (else
      (`self.K2_EndAbility`))))

(event `self.K2_OnEndAbility`
  (params (bWasCancelled :type Boolean))
  (if bWasCancelled
    (`CharacterMovementComponent.SetMovementMode` (`Character.CharacterMovement` (`self.Player`)) "MOVE_Walking" 0)))