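; Basic melee attack Gameplay Ability shared by the player character and AI, branching on the avatar's "Player" tag.
; After committing, it plays the damage montage and waits once for an Action.Damage gameplay event.
; The event applies GE_MeleDamage from instigator to target, with Damage passed as a SetByCaller magnitude.
; AI hits land only on non-blocking player characters and end the ability; montage completion or interruption clears IsAttacking.
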(event `self.K2_ActivateAbility`
  (bind _returnvalue (`self.GetAvatarActorFromActorInfo`))
  (if (`Actor.ActorHasTag` _returnvalue "Player")
    (bind _asbp_my_character (cast `/Game/Bluprints/BP_MyCharacter` _returnvalue))
    (set `self.Player` _asbp_my_character)
    (bind _returnvalue_2 (`self.K2_CommitAbility`))
    (if _returnvalue_2
      (`AbilityTask_PlayMontageAndWait.CreatePlayMontageAndWaitProxy` "None" (`self.Damage Montage`)
        (:`then`
          (bind (_asynctaskproxy _payload) (`AbilityTask_WaitGameplayEvent.WaitGameplayEvent` (struct :`TagName` "Action.Damage") null true)
            (:`EventReceived`
              (bind _result (`/Engine/EditorBlueprintResources/StandardMacros.NegateFloat` (`self.Damage`))
                (:`  `
                  (bind _returnvalue_3 (`AbilitySystemBlueprintLibrary.AssignTagSetByCallerMagnitude` (`self.MakeOutgoingGameplayEffectSpec` "/Game/GAS/Effects/GE_MeleDamage.GE_MeleDamage_C") (struct :`TagName` "Action.Damage") _result))
                  (bind (_eventtag _instigator _target) (break `GameplayEventData` _payload))
                  (`AbilitySystemComponent.BP_ApplyGameplayEffectSpecToTarget` (`AbilitySystemBlueprintLibrary.GetAbilitySystemComponent` _instigator) _returnvalue_3 (`AbilitySystemBlueprintLibrary.GetAbilitySystemComponent` _target)))))))
        (:`OnCompleted`
          (`self.K2_EndAbility` :!label _label))
        (:`OnBlendOut`
          (goto _label))
        (:`OnInterrupted`
          (goto _label))
        (:`OnCancelled`
          (goto _label)))
      (else
        (`self.K2_EndAbility`)))
    (else
      (bind _asbp_ai_01 (cast `/Game/AI/BP_AI_01` _returnvalue))
      (set `self.AI` _asbp_ai_01)
      (bind _returnvalue_4 (`self.K2_CommitAbility`))
      (if _returnvalue_4
        (`AbilityTask_PlayMontageAndWait.CreatePlayMontageAndWaitProxy` "None" (`self.Damage Montage`)
          (:`then`
            (bind (_asynctaskproxy_2 _payload_2) (`AbilityTask_WaitGameplayEvent.WaitGameplayEvent` (struct :`TagName` "Action.Damage") null true)
              (:`EventReceived`
                (bind (_eventtag_2 _instigator_2 _target_2) (break `GameplayEventData` _payload_2))
                (bind _asbp_my_character_2 (cast `/Game/Bluprints/BP_MyCharacter` _target_2))
                (bind _result_2 (`/Engine/EditorBlueprintResources/StandardMacros.NegateFloat` (`self.Damage`))
                  (:`  `
                    (bind _returnvalue_5 (`AbilitySystemBlueprintLibrary.AssignTagSetByCallerMagnitude` (`self.MakeOutgoingGameplayEffectSpec` "/Game/GAS/Effects/GE_MeleDamage.GE_MeleDamage_C") (struct :`TagName` "Action.Damage") _result_2))
                    (if (not (`MyCharacter.is_block` _asbp_my_character_2))
                      (`AbilitySystemComponent.BP_ApplyGameplayEffectSpecToTarget` (`AbilitySystemBlueprintLibrary.GetAbilitySystemComponent` _instigator_2) _returnvalue_5 (`AbilitySystemBlueprintLibrary.GetAbilitySystemComponent` _target_2))
                      (`self.K2_EndAbility`)))))))
          (:`OnCompleted`
            (set `/Game/AI/BP_AI_01.isAttacking?` false (`self.AI`) :!label _label_2)
            (`self.K2_EndAbility`))
          (:`OnInterrupted`
            (goto _label_2)))
        (else
          (`self.K2_EndAbility`))))))